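; Race gate actor that a FlyingPawn passes through in order along a course.
; When flagged as next, its box overlap advances the pawn's gate count, clears the flag and restores the passive color.
; The first gate starts the pawn's timer and the last, found from the GateArray length on the pawn's DrawingCharRef, stops it.
; A dynamic material instance created on BeginPlay drives the color.
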(event `self.ReceiveBeginPlay`
  (bind _returnvalue (`PrimitiveComponent.CreateDynamicMaterialInstance` (`self.StaticMesh`) 0 "/Game/Materials/GateMaterials/Emmisive.Emmisive"))
  (bind _output_get (set `self.DynamicMat` _returnvalue))
  (`MaterialInstanceDynamic.SetVectorParameterValue` _output_get "Color" (`self.PassiveColor`)))

(event `self.Box.OnComponentBeginOverlap`
  (params (OverlappedComponent :type "PrimitiveComponent Object Reference") (OtherActor :type "Actor Object Reference") (OtherComp :type "PrimitiveComponent Object Reference") (OtherBodyIndex :type Integer) (bFromSweep :type Boolean) (SweepResult :type "HitResult Structure (by ref)"))
  (bind _order (`self.Order`))
  (if (`self.bNext`)
    (bind _asflying_pawn (cast `/Game/Core/Blueprints/FlyingPawn` OtherActor))
    (if (== _order 0)
      (`/Game/Core/Blueprints/FlyingPawn.StartTimer` _asflying_pawn)
      (elif (== _order (- (`KismetArrayLibrary.Array_Length` (`/Game/Core/Blueprints/DrawingPawn.GateArray` (`/Game/Core/Blueprints/FlyingPawn.DrawingCharRef` _asflying_pawn))) 1))
        (`/Game/Core/Blueprints/FlyingPawn.StopTimer` _asflying_pawn)))
    (`/Game/Core/Blueprints/FlyingPawn.IncrementGate` _asflying_pawn)
    (`MaterialInstanceDynamic.SetVectorParameterValue` (`self.DynamicMat`) "Color" (`self.PassiveColor`))
    (set `self.bNext` false)))

(event `self.StaticMesh.OnComponentBeginOverlap`
  (params (OverlappedComponent :type "PrimitiveComponent Object Reference") (OtherActor :type "Actor Object Reference") (OtherComp :type "PrimitiveComponent Object Reference") (OtherBodyIndex :type Integer) (bFromSweep :type Boolean) (SweepResult :type "HitResult Structure (by ref)")))

(fn `UserConstructionScript`)